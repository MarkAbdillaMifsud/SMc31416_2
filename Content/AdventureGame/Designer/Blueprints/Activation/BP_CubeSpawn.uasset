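; BP_CubeSpawn is a switch-activated spawner that creates a BP_Cube at its own transform.
; FnBPISwitchon spawns only while CanSpawn is set, then clears that flag.
; Once CubesSpawned reaches MaxNumCubes, each spawn first destroys the oldest cube in SpawnedCubes; the counter never decreases.
; EvResetSpawn re-arms CanSpawn in a self-calling Delay loop using SpawnCooldown, but nothing in this file starts it.
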(event Custom|EvResetSpawn
  (Utilities|FlowControl|Delay (Variables|Setup|GetSpawnCooldown))
  (Variables|Default|SetCanSpawn true)
  (CallFunction|EvResetSpawn))

(event EventBeginPlay)

(event Collision|EventActorBeginOverlap
  (params (OtherActor :type Actor%20Object%20Reference)))

(event EventTick
  (params (DeltaSeconds :type Float%20%28single-precision%29)))

(event EventFnBPISwitchon
  (bind _returnvalue (Transformation|GetActorTransform))
  (if (Variables|Default|GetCanSpawn)
    (if (< (Variables|Default|GetCubesSpawned) (Variables|Setup|GetMaxNumCubes))
      _
      (else
        (Actor|DestroyActor (Utilities|Array|Get(acopy) (Variables|Default|GetSpawnedCubes)))
        (Utilities|Array|RemoveIndex (Variables|Default|GetSpawnedCubes))))
    (Math|Integer|IncrementInt (Variables|Default|GetCubesSpawned)
      (:%20%20
        (bind _returnvalue_2 (Game|SpawnActorfromClass "/Game/AdventureGame/Designer/Blueprints/Activation/BP_Cube.BP_Cube_C" (Math|Transform|MakeTransform (.location _returnvalue) (.rotation _returnvalue) (.scale _returnvalue)) "Undefined" "MultiplyWithRoot" 0 0))
        (Utilities|Array|Add (Variables|Default|GetSpawnedCubes) _returnvalue_2)
        (Variables|Default|SetCanSpawn false)))))

(fn ConstructionScript)