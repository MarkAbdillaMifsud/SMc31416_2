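; BP_Switch is a trigger-driven switch that activates a list of linked objects when something overlaps it.
; On overlap it swaps the switch mesh to the on material and sends each listed object a switch-on interface message.
; Unless set to activate once, it reverts material and sends switch-off messages only when the last overlapping actor leaves.
; The construction script starts it in the off material.
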(event OnComponentBeginOverlap(Trigger)
  (params (OverlappedComponent :type Primitive%20Component%20Object%20Reference) (OtherActor :type Actor%20Object%20Reference) (OtherComp :type Primitive%20Component%20Object%20Reference) (OtherBodyIndex :type Integer) (bFromSweep :type Boolean) (SweepResult :type Hit%20Result%20Structure%20%28by%20ref%29))
  (Rendering|Material|SetMaterial (Variables|Default|GetSwitch) 0 (Variables|Setup|GetOnMaterial))
  (for _array_element (Variables|Setup|GetInteractObjectList)
    (Class|BPIInteraction|FnBPISwitchon(Message) _array_element)))

(event OnComponentEndOverlap(Trigger)
  (params (OverlappedComponent :type Primitive%20Component%20Object%20Reference) (OtherActor :type Actor%20Object%20Reference) (OtherComp :type Primitive%20Component%20Object%20Reference) (OtherBodyIndex :type Integer))
  (if (not (Variables|Setup|GetActivateOnce))
    (if (Utilities|Array|IsEmpty (Collision|GetOverlappingActors (Variables|Default|GetTrigger) 0 :!class /Script/Engine.PrimitiveComponent))
      (Rendering|Material|SetMaterial (Variables|Default|GetSwitch) 0 (Variables|Setup|GetOffMaterial))
      (for _array_element (Variables|Setup|GetInteractObjectList)
        (Class|BPIInteraction|FnBPISwitchOff(Message) _array_element)))))

(fn ConstructionScript
  (Rendering|Material|SetMaterial (Variables|Default|GetSwitch) 0 (Variables|Setup|GetOffMaterial)))