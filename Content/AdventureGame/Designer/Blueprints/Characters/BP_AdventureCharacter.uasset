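; Player character for the adventure game that tracks health and held keys and handles elimination.
; On possession it creates the player HUD, which updates as damage is taken or keys are added through interface-style functions.
; At zero health a DoOnce disables input, shows the eliminated screen and reloads the current level after a short delay.
; The weapon target location function is a stub returning the zero vector.
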(event EventBeginPlay)

(event Collision|EventActorBeginOverlap
  (params (OtherActor :type Actor%20Object%20Reference)))

(event EventTick
  (params (DeltaSeconds :type Float%20%28single-precision%29)))

(event EventFnBPIAddKey
  (params (KeyType :type Enum_KeyType%20Enum :default "NewEnumerator0"))
  (Utilities|Array|Add (Variables|Default|GetHeld%20Keys) KeyType)
  (Default|FnAddKeyHUD (Variables|Default|GetHUD) KeyType))

(event EventPossessed
  (params (NewController :type Controller%20Object%20Reference))
  (|CallParentFunction NewController)
  (bind _returnvalue (UserInterface|CreateWidget "/Game/AdventureGame/Designer/Blueprints/Widgets/WBP_PlayerHUD.WBP_PlayerHUD_C"))
  (bind _output_get (Variables|Default|SetHUD _returnvalue))
  (Default|FnSetHP _output_get (Variables|Default|GetHealth))
  (UserInterface|Viewport|AddtoViewport (Variables|Default|GetHUD) 0))

(event Game|Damage|EventAnyDamage
  (params (Damage :type Float%20%28single-precision%29) (DamageType :type Damage%20Type%20Object%20Reference) (InstigatedBy :type Controller%20Object%20Reference) (DamageCauser :type Actor%20Object%20Reference))
  (bind _output_get (Variables|Default|SetHealth (- (Variables|Default|GetHealth) Damage)))
  (if (<= _output_get 0.0)
    (Utilities|FlowControl|DoOnce false
      (:Completed
        (Input|DisableInput (Game|GetPlayerController 0))
        (bind _returnvalue (UserInterface|CreateWidget "/Game/AdventureGame/Designer/Blueprints/Widgets/WBP_EliminatedScreen.WBP_EliminatedScreen_C"))
        (UserInterface|Viewport|AddtoViewport _returnvalue 0)
        (Utilities|FlowControl|Delay 5.0)
        (bind _returnvalue_2 (Game|GetCurrentLevelName true))
        (Game|OpenLevel(byName) (Utilities|String|StringToName _returnvalue_2))))
    (else
      (Default|FnSetHP (Variables|Default|GetHUD) (Variables|Default|GetHealth)))))

(fn ConstructionScript)

(fn FnBPIGetKeys
  (return (Variables|Default|GetHeld%20Keys)))

(fn GetWeaponTargetLocation
  (return "0, 0, 0"))