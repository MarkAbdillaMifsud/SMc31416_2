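; Blueprint function library for the first-person adventure game, with helpers for key visuals and player detection.
; The key helper looks up a key in a map and applies its material, plus its mesh when valid, to an array of static meshes.
; The detection helper returns true when a Camera-channel line trace hits the player within a maximum distance, with optional debug drawing.
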(fn FnBPLSetKey
  (params (Static%20Mesh%20Array :type Array%20of%20Static%20Mesh%20Component%20Object%20References) (KeyMap :type Map%20of%20Enum_KeyType%20Enums%20to%20Structs :default "NewEnumerator0") (Key :type Enum_KeyType%20Enum :default "NewEnumerator0"))
  (bind _value (Utilities|Map|Find KeyMap Key))
  (for _array_element Static%20Mesh%20Array
    (Utilities|IsValid (.keymesh _value)
      (:Is%20Valid
        (Components|StaticMesh|SetStaticMesh _array_element (.keymesh _value)))
      (:Is%20Not%20Valid
        _))
    (Rendering|Material|SetMaterial _array_element 0 (.keymaterial _value))))

(fn FnBPLFindPlayer
  (params (Player%20Reference :type Pawn%20Object%20Reference) (Start%20Location :type Vector) (Max%20Detection%20Distance :type Float%20%28double-precision%29) (Debug :type Boolean))
  (Utilities|IsValid Player%20Reference
    (:Is%20Valid
      (Utilities|FlowControl|Sequence
        (:then_0
          (bind _outhit (Collision|LineTraceByChannel 0 Start%20Location (Transformation|GetActorLocation Player%20Reference) "TraceTypeQuery2" false 0 (select Debug "ForDuration" "None") true "(R=1.000000,G=0.000000,B=0.000000,A=1.000000)" "(R=0.000000,G=1.000000,B=0.000000,A=1.000000)" 0.1))
          (if (and (== (.HitActor (Collision|BreakHitResult _outhit)) Player%20Reference) (< (Math|Vector|Distance(Vector) (.TraceStart (Collision|BreakHitResult _outhit)) (.TraceEnd (Collision|BreakHitResult _outhit))) Max%20Detection%20Distance))
            (return true)
            (else
              (LocalVariables|SetPlayerFound false))))
        (:then_1
          (return false))))
    (:Is%20Not%20Valid
      (return false))))