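; BP_FinalRoomManager tracks the enemies in the final room and activates a jump pad once all are eliminated.
; On BeginPlay it counts the RoomEnemies array and binds a handler to each enemy's OnEnemyEliminated event.
; Each elimination decrements the remaining count, printing it for debugging, and at zero it calls ActivateJumpPad on the referenced jump pad.
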(event Custom|HandleEnemyEliminated
  (bind _output_get (Variables|Default|SetRemainingEnemies (- (Variables|Default|GetRemainingEnemies) 1)))
  (Development|PrintString (Utilities|String|ToString(Integer) _output_get))
  (if (<= (Variables|Default|GetRemainingEnemies) 0)
    (Default|ActivateJumpPad (Variables|Default|GetJumpPadRef))))

(event EventBeginPlay
  (bind _output_get (Variables|Default|SetRemainingEnemies (Utilities|Array|Length (Variables|Default|GetRoomEnemies))))
  (Development|PrintString (Utilities|String|ToString(Integer) _output_get))
  (for _array_element (Variables|Default|GetRoomEnemies)
    (EventDispatchers|BindEventtoOnEnemyEliminated _array_element (delegate Custom|HandleEnemyEliminated))))

(event Collision|EventActorBeginOverlap
  (params (OtherActor :type Actor%20Object%20Reference)))

(event EventTick
  (params (DeltaSeconds :type Float%20%28single-precision%29)))

(fn ConstructionScript)