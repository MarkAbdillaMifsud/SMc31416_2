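; BP_Platform is a switch-controlled moving platform that shuttles between its starting location and a TargetPoint while active.
; A timeline, rate-scaled by TimeToTarget, lerps the mesh position, then waits WaitDuration and reverses if still active.
; Switch-on interface events start it forward; switch-off sends it back to the start to rest.
; An optional AttachedKey rides along, and the construction script applies PlatformScale.
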(event Custom|evMoveForward
  (bind (_direction _alpha) (Timeline|TM_MovePlatform Play)
    (:Update
      (Transformation|SetWorldLocation (Variables|Default|GetPlatform) (Math|Vector|Lerp(Vector) (Variables|Default|GetStartLocation) (Variables|Default|GetEndLocation) _alpha) false false))
    (:Finished
      (Utilities|FlowControl|Delay (Variables|Setup|GetWaitDuration))
      (if (Variables|Setup|GetActive)
        (if (Utilities|Enum|Equal(Enum) _direction "Forward")
          (CallFunction|EvMoveBackward)
          (else
            (CallFunction|EvMoveForward)))))))

(event Custom|evMoveBackward
  (bind (_direction _alpha) (Timeline|TM_MovePlatform Reverse)
    (:Update
      (Transformation|SetWorldLocation (Variables|Default|GetPlatform) (Math|Vector|Lerp(Vector) (Variables|Default|GetStartLocation) (Variables|Default|GetEndLocation) _alpha) false false))
    (:Finished
      (Utilities|FlowControl|Delay (Variables|Setup|GetWaitDuration))
      (if (Variables|Setup|GetActive)
        (if (Utilities|Enum|Equal(Enum) _direction "Forward")
          (CallFunction|EvMoveBackward)
          (else
            (CallFunction|EvMoveForward)))))))

(event Custom|evStop
  (bind (_direction _alpha) (Timeline|TM_MovePlatform Stop)
    (:Update
      (Transformation|SetWorldLocation (Variables|Default|GetPlatform) (Math|Vector|Lerp(Vector) (Variables|Default|GetStartLocation) (Variables|Default|GetEndLocation) _alpha) false false))
    (:Finished
      (Utilities|FlowControl|Delay (Variables|Setup|GetWaitDuration))
      (if (Variables|Setup|GetActive)
        (if (Utilities|Enum|Equal(Enum) _direction "Forward")
          (CallFunction|EvMoveBackward)
          (else
            (CallFunction|EvMoveForward)))))))

(event EventBeginPlay
  (Utilities|IsValid (Variables|Default|GetAttachedKey)
    (:Is%20Valid
      (Transformation|AttachComponentToComponent (Variables|Default|GetAttachedKey) (Variables|Default|GetPlatform) "None" "KeepWorld" "KeepWorld" "KeepWorld" true))
    (:Is%20Not%20Valid
      _))
  (Variables|Default|SetStartLocation (Transformation|GetActorLocation))
  (Variables|Default|SetEndLocation (Transformation|GetActorLocation (Variables|Setup|GetTargetPoint)))
  (Components|Timeline|SetPlayRate (Variables|Default|GetTM_MovePlatform) (/ 1.0 (Variables|Setup|GetTimeToTarget))))

(event EventFnBPISwitchon
  (Variables|Setup|SetActive true)
  (CallFunction|EvMoveForward))

(event EventFnBPISwitchOff
  (Variables|Setup|SetActive false)
  (CallFunction|EvMoveBackward))

(fn ConstructionScript
  (Transformation|SetWorldScale3D (Variables|Default|GetPlatform) (Variables|Setup|GetPlatformScale)))