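; BP_TrapFire is a fire trap Blueprint that responds to switch interface events.
; Switch-on clears Active and applies OffMaterial to TrapBase, while switch-off sets Active and applies OnMaterial, so the trap runs inverse to its switch.
; BeginPlay, overlap and Tick are disabled stubs, and the construction script only calls its parent, so this graph holds no damage or effect logic.
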(event EventBeginPlay
  (|CallParentFunction) ; This node is disabled and will not be called.\nDrag off pins to build functionality.
)

(event Collision|EventActorBeginOverlap
  (params (OtherActor :type Actor%20Object%20Reference)))

(event EventTick
  (params (DeltaSeconds :type Float%20%28single-precision%29)))

(event EventFnBPISwitchon
  (Variables|Default|SetActive false)
  (Rendering|Material|SetMaterial (Variables|Default|GetTrapBase) 0 (Variables|Setup|GetOffMaterial)))

(event EventFnBPISwitchOff
  (Variables|Default|SetActive true)
  (Rendering|Material|SetMaterial (Variables|Default|GetTrapBase) 0 (Variables|Setup|GetOnMaterial)))

(fn ConstructionScript
  (|CallParentFunction))